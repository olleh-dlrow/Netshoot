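; Timer actor that runs the match countdown for a two-player networked gunslinger game.
; On authority, Tick waits for two Gunslinger_BP actors, starts a short countdown, then triggers game end when it expires.
; ClientGameEnd receives the PlayerArray and, on remotes, shows a one-time end widget with both player states and the mouse cursor.
; ClientGameStart can show a start widget but is not called here, and the time RepNotify is empty.
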(event Custom|ClientGameStart
  (Networking|SwitchHasAuthority
    (:Remote
      (Development|PrintString "Game Start")
      (bind _returnvalue (UserInterface|CreateWidget "/Game/Blueprints/Widgets/GameStart.GameStart_C" (Game|GetPlayerController 0)))
      (UserInterface|Viewport|AddtoViewport _returnvalue 0))))

(event Custom|GameEnd
  (Networking|SwitchHasAuthority
    (:Authority
      (CallFunction|ClientGameEnd (Variables|/Script/Engine.GameStateBase|GetPlayerArray (Game|GetGameState))))))

(event Custom|ClientGameEnd
  (params (PlayerArray :type Array%20of%20Player%20State%20Object%20References))
  (if (not (Variables|Default|GetinViewPort))
    (Networking|SwitchHasAuthority
      (:Remote
        (bind _returnvalue (UserInterface|CreateWidget "/Game/Blueprints/Widgets/GameEndWidget.GameEndWidget_C" (Game|GetPlayerController 0)))
        (bind _asmy_player_state (Utilities|Casting|CastToMyPlayerState (Utilities|Array|Get(acopy) PlayerArray)))
        (Variables|/Game/Blueprints/Widgets/GameEndWidget.GameEndWidget_C|SetPlayerState1 _returnvalue _asmy_player_state)
        (bind _asmy_player_state_2 (Utilities|Casting|CastToMyPlayerState (Utilities|Array|Get(acopy) PlayerArray 1)))
        (Variables|/Game/Blueprints/Widgets/GameEndWidget.GameEndWidget_C|SetPlayerState2 _returnvalue _asmy_player_state_2)
        (UserInterface|Viewport|AddtoViewport _returnvalue 0)
        (Variables|Default|SetinViewPort true)
        (Variables|/Script/Engine.PlayerController|SetbShowMouseCursor (Game|GetPlayerController 0) true)))))

(event EventBeginPlay)

(event EventTick
  (params (DeltaSeconds :type Float%20%28single-precision%29))
  (if (not (Variables|Default|GetbGameEnd))
    (Networking|SwitchHasAuthority
      (:Authority
        (if (Variables|Default|GetbGameStart)
          (bind _output_get (Variables|Default|SetcurTime (- (Variables|Default|GetcurTime) DeltaSeconds)))
          (if (<= (Math|Float|Truncate _output_get) 0)
            (Variables|Default|SetbGameEnd true)
            (CallFunction|GameEnd))
          (else
            (bind _outactors (Actor|GetAllActorsOfClass "/Game/Gunslinger/Gunslinger_BP.Gunslinger_BP_C"))
            (if (== (Utilities|Array|Length _outactors) 2)
              (Variables|Default|SetbGameStart true)
              (Variables|Default|SetcurTime 1e+01))))))))

(fn ConstructionScript)

(fn OnRepCurTime)