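; Cube_BP is a flying cube actor that bobs up and down continuously in the level.
; Each Tick it offsets its world position along Z by a fixed step scaled by a Dir variable, without sweep or delta-time scaling, so speed depends on frame rate.
; Dir flips to downward above an upper world-height limit and back to upward below a lower one.
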(event EventBeginPlay)

(event Collision|EventActorBeginOverlap
  (params (OtherActor :type Actor%20Object%20Reference)))

(event EventTick
  (params (DeltaSeconds :type Float%20%28single-precision%29))
  (bind _returnvalue (Transformation|GetActorLocation))
  (bind _z (Math|Vector|BreakVector _returnvalue))
  (Transformation|AddActorWorldOffset (Math|Vector|MakeVector 0.0 0.0 (* (Variables|Default|GetDir) 5.0)))
  (if (> _z 3e+02)
    (Variables|Default|SetDir -1)
    (elif (< _z 1.5e+02)
      (Variables|Default|SetDir 1))))

(fn ConstructionScript)