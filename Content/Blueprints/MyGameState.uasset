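; Game state that runs a timed round for the match and shows the start and end screens.
; On authority, Tick starts the countdown once MyGameMode has players and ends the round at zero.
; GameEnd resets the round and player count, then passes PlayerArray to ClientGameEnd, which shows a results widget for the first two player states.
; ClientGameStart adds a start widget on remotes but is not called here.
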(event Custom|ClientGameStart
  (Networking|SwitchHasAuthority
    (:Remote
      (bind _returnvalue (UserInterface|CreateWidget "/Game/Blueprints/Widgets/GameStart.GameStart_C" (Game|GetPlayerController 0)))
      (UserInterface|Viewport|AddtoViewport _returnvalue 0))))

(event Custom|GameEnd
  (Networking|SwitchHasAuthority
    (:Authority
      (Variables|Default|SetCurTime (Variables|Default|GetMaxTime))
      (Variables|Default|SetbInViewPort false)
      (Variables|Default|SetbGameEnd false)
      (Variables|Default|SetbGameStart false)
      (bind _asmy_game_mode (Utilities|Casting|CastToMyGameMode (Game|GetGameMode)))
      (Variables|/Game/Blueprints/MyGameMode.MyGameMode_C|SetPlayerCount _asmy_game_mode 0)
      (CallFunction|ClientGameEnd (Variables|/Script/Engine.GameStateBase|GetPlayerArray (Game|GetGameState))))))

(event Custom|ClientGameEnd
  (params (PlayerArray :type Array%20of%20Player%20State%20Object%20References))
  (if (not (Variables|Default|GetbInViewPort))
    (Networking|SwitchHasAuthority
      (:Authority
        _)
      (:Remote
        _))
    (bind _returnvalue (UserInterface|CreateWidget "/Game/Blueprints/Widgets/GameEndWidget.GameEndWidget_C" (Game|GetPlayerController 0)))
    (bind _asmy_player_state (Utilities|Casting|CastToMyPlayerState (Utilities|Array|Get(acopy) PlayerArray))
      (:then
        (Variables|/Game/Blueprints/Widgets/GameEndWidget.GameEndWidget_C|SetPlayerState1 _returnvalue _asmy_player_state)
        (bind _asmy_player_state_2 (Utilities|Casting|CastToMyPlayerState (Utilities|Array|Get(acopy) PlayerArray 1))
          (:then
            (Variables|/Game/Blueprints/Widgets/GameEndWidget.GameEndWidget_C|SetPlayerState2 _returnvalue _asmy_player_state_2))
          (:CastFailed
            _)))
      (:CastFailed
        _))
    (UserInterface|Viewport|AddtoViewport _returnvalue 0)
    (Variables|Default|SetbInViewPort true)
    (Variables|/Script/Engine.PlayerController|SetbShowMouseCursor (Game|GetPlayerController 0) true)))

(event EventTick
  (params (DeltaSeconds :type Float%20%28single-precision%29))
  (if (not (Variables|Default|GetbGameEnd))
    (Networking|SwitchHasAuthority
      (:Authority
        (if (Variables|Default|GetbGameStart)
          (bind _output_get (Variables|Default|SetcurTime (- (Variables|Default|GetcurTime) DeltaSeconds)))
          (if (<= (Math|Float|Truncate _output_get) 0)
            (Variables|Default|SetbGameEnd true)
            (CallFunction|GameEnd))
          (else
            (bind _asmy_game_mode (Utilities|Casting|CastToMyGameMode (Game|GetGameMode)))
            (if (> (Variables|/Game/Blueprints/MyGameMode.MyGameMode_C|GetPlayerCount _asmy_game_mode) 0)
              (Variables|Default|SetbGameStart true)
              (Variables|Default|SetcurTime (Variables|Default|GetMaxTime)))))))))

(event EventBeginPlay
  (Networking|SwitchHasAuthority
    (:Authority
      (Variables|Default|SetCurTime (Variables|Default|GetMaxTime))
      (Variables|Default|SetbInViewPort false)
      (Variables|Default|SetbGameEnd false)
      (Variables|Default|SetbGameStart false))))

(fn ConstructionScript)

(fn OnRepGameStartTimer)

(fn OnRepRandomTimerValue1)