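; Server-authoritative spawner actor that keeps a fixed set of FlyObject_BP actors populated at predefined locations.
; On BeginPlay it spawns one object at each of the first four FlyObjLocations, hands each its spawner and slot index, and stores it in FlyObjects.
; A looping timer, set inside that spawn loop, periodically scans the array and refills any empty slot at its matching location.
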(event Custom|ReSpawnFlyobj
  (Networking|SwitchHasAuthority
    (:Authority
      (for (_array_element _array_index) (Variables|Default|GetFlyObjects)
        (if (== _array_element 0)
          (bind _returnvalue (Game|SpawnActorfromClass "/Game/Blueprints/FlyObject/FlyObject_BP.FlyObject_BP_C" (Math|Conversions|ToTransform(Vector) (Utilities|Array|Get(acopy) (Variables|Default|GetFlyObjLocations) _array_index)) "Undefined" 0 0))
          (Variables|/Game/Blueprints/FlyObject/FlyObject_BP.FlyObject_BP_C|SetSpawner _returnvalue self)
          (bind _output_get (Variables|/Game/Blueprints/FlyObject/FlyObject_BP.FlyObject_BP_C|Setindex _returnvalue _array_index))
          (Utilities|Array|SetArrayElem (Variables|Default|GetFlyObjects) _output_get _returnvalue))))))

(event EventBeginPlay
  (Networking|SwitchHasAuthority
    (:Authority
      (for _index (range 0 3)
        (bind _returnvalue (Game|SpawnActorfromClass "/Game/Blueprints/FlyObject/FlyObject_BP.FlyObject_BP_C" (Math|Transform|MakeTransform (Utilities|Array|Get(acopy) (Variables|Default|GetFlyObjLocations) _index)) "Undefined" 0 0))
        (Variables|/Game/Blueprints/FlyObject/FlyObject_BP.FlyObject_BP_C|SetSpawner _returnvalue self)
        (Variables|/Game/Blueprints/FlyObject/FlyObject_BP.FlyObject_BP_C|Setindex _returnvalue _index)
        (Utilities|Array|SetArrayElem (Variables|Default|GetFlyObjects) _index _returnvalue)
        (Utilities|Time|SetTimerbyEvent (delegate Custom|ReSpawnFlyobj) 5.0 true)))))

(fn ConstructionScript)